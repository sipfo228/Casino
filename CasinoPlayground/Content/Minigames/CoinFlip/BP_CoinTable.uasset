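; Interactable coin-flip minigame table where the player picks heads or tails and throws a coin to win or lose.
; BeginInteraction opens the coin game UI with a mouse cursor and binds its buttons; picking a side spawns a BP_Coin above the table if none exists.
; Throwing waits a fixed delay, then, if the coin is still, compares its up face to the chosen side, shows the result and re-enables side selection.
; EndInteraction destroys the coin.
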(event `OnClickThrow_Event`
  (bind _gameui (`self.GameUI`))
  (bind _gameui_2 (`self.GameUI`))
  (bind _roll (`/Game/Minigames/CoinFlip/BP_CoinGameUI.Roll` _gameui))
  ; Spawn Ground Check
  (`/Engine/EditorBlueprintResources/StandardMacros.CompareInt` (`self.CoinGrounded`) 1
    (:`==`
      (for _ (range 1)
        (`/Game/Minigames/CoinFlip/BP_Coin.Throw` (`self.CoinRef`))
        (`KismetSystemLibrary.Delay` 2.0)
        ; Result Check
        (if (not (> (`KismetMathLibrary.VSize` (`self.GetVelocity` (`self.CoinRef`))) 0.1))
          (set `self.CoinGrounded` 1)
          (`KismetSystemLibrary.PrintString` "stopped")
          (if (`KismetStringLibrary.EqualEqual_StrStr` (`/Game/Minigames/CoinFlip/BP_CoinGameUI.ChoosedSide` (`self.GameUI`)) (`/Game/Minigames/CoinFlip/BP_Coin.UpFace` (`self.CoinRef`)))
            (set `self.WinCond` true)
            (`/Game/Minigames/CoinFlip/BP_CoinGameUI.Update Result` _gameui_2 "Big Win!")
            (else
              (set `self.WinCond` false)
              (`/Game/Minigames/CoinFlip/BP_CoinGameUI.Update Result` _gameui_2 "Massive Lose")))
          ; Enable face selection
          (`Widget.SetIsEnabled` (`/Game/Minigames/CoinFlip/BP_CoinGameUI.Tails` _gameui) true)
          (`Widget.SetIsEnabled` (`/Game/Minigames/CoinFlip/BP_CoinGameUI.Heads` _gameui) true)
          (`Widget.SetVisibility` (`/Game/Minigames/CoinFlip/BP_CoinGameUI.Heads` _gameui) "Visible")
          (`Widget.SetVisibility` (`/Game/Minigames/CoinFlip/BP_CoinGameUI.Tails` _gameui) "Visible")
          (`Widget.SetIsEnabled` _roll false)
          (`Widget.SetVisibility` _roll "Hidden")))
      (set `self.CoinGrounded` 0))))

(event `self.BeginInteraction`
  (bind _returnvalue (`GameplayStatics.GetPlayerController` 0))
  (bind _gameui (`self.GameUI`))
  (`parent.BeginInteraction`)
  ; Camera and UI setup
  (if (not (`Widget.IsInViewport` (stale _returnvalue_2)))
    (bind _returnvalue_2 (`|CreateWidget` "/Game/Minigames/CoinFlip/BP_CoinGameUI.BP_CoinGameUI_C" _returnvalue))
    (bind _output_get (set `self.GameUI` _returnvalue_2))
    (`UserWidget.AddToViewport` _output_get 0)
    (`WidgetBlueprintLibrary.SetFocusToGameViewport`)
    (set `PlayerController.bShowMouseCursor` true _returnvalue)
    (add `/Game/Minigames/CoinFlip/BP_CoinGameUI.OnClickThrow` _gameui (delegate `OnClickThrow_Event`))
    (add `/Game/Minigames/CoinFlip/BP_CoinGameUI.OnClickHeads` _gameui (delegate `OnClickHeads_Event`))
    (add `/Game/Minigames/CoinFlip/BP_CoinGameUI.OnClickTails` _gameui (delegate `OnClickTails_Event`))))

(event `OnClickTails_Event`
  ; Spawn coin on side selection
  (bind _returnvalue (`GameplayStatics.GetActorOfClass` "/Game/Minigames/CoinFlip/BP_Coin.BP_Coin_C" :!label _label))
  (`/Engine/EditorBlueprintResources/StandardMacros.IsValid` _returnvalue
    (:`Is Not Valid`
      (bind _returnvalue_2 (`|SpawnActorFromClass` "/Game/Minigames/CoinFlip/BP_Coin.BP_Coin_C" (`KismetMathLibrary.Conv_VectorToTransform` (+ (`self.K2_GetActorLocation`) (-30.0 -30.0 170.0))) "Undefined" "MultiplyWithRoot" null null))
      (set `self.CoinRef` _returnvalue_2))))

(event `OnClickHeads_Event`
  ; Spawn coin on side selection
  (goto _label))

(event `self.EndInteraction`
  ; Destroy Coin on Exit
  (`self.K2_DestroyActor` (`self.CoinRef`))
  (set `self.CoinRef` null))

(fn `UserConstructionScript`
  (`parent.UserConstructionScript`))