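; Goblet actor for the goblet-pick minigame that slides along the table's splines when shuffled.
; On BeginPlay it finds BP_GobletTable, and FindPossibleSplines collects the table splines passing close to the goblet.
; Shuffle moves it along ChoosedSpline with a timeline, played forward or reversed, tracking IsStopped.
; Spline selection is not done in live code here; several disconnected experiments remain in the graph.
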(event `self.ReceiveActorBeginOverlap`
  (params (OtherActor :type "Actor Object Reference")))

(event `OnStop`)

(event `self.ReceiveBeginPlay`
  ; Get Spline Refs
  (set `self.IsStopped` true)
  (if (== (`self.TableRef`) null)
    (bind _returnvalue (`GameplayStatics.GetActorOfClass` "/Game/Minigames/GobletPick/BP_GobletTable.BP_GobletTable_C"))
    (set `self.TableRef` _returnvalue)
    (`KismetArrayLibrary.Array_Clear` (`self.FoundSplineRefs`))))

(event `FindPossibleSplines`
  (bind _returnvalue (`self.K2_GetActorLocation`))
  ; Find possible splines to move
  (`KismetArrayLibrary.Array_Clear` (`self.FoundSplineRefs`))
  (for _array_element (`self.K2_GetComponentsByClass` (`self.TableRef`) "/Script/Engine.SplineComponent")
    (if (< (`KismetMathLibrary.Vector_Distance` (`SplineComponent.GetLocationAtSplineInputKey` _array_element (`SplineComponent.FindInputKeyClosestToWorldLocation` _array_element _returnvalue) "World") _returnvalue) 20.0)
      (`KismetArrayLibrary.Array_Add` (`self.FoundSplineRefs`) _array_element))))

(event `self.ReceiveEndPlay`
  (params (EndPlayReason :type "EEndPlayReason Enum" :default "Destroyed"))
  ; Clear after exiting
  (set `self.ChoosedSpline` null)
  (set `self.MovementDir` null)
  (set `self.TableRef` null)
  (`KismetArrayLibrary.Array_Clear` (`self.AllSplineRefs`))
  (`KismetArrayLibrary.Array_Clear` (`self.FoundSplineRefs`))
  (set `self.StartPointDist` 0.0))

(event `Shuffle`
  (bind _choosedspline (`self.ChoosedSpline`))
  (bind _startpointdist (`self.StartPointDist`))
  (bind _choosedspline_2 (`self.ChoosedSpline`))
  (bind _returnvalue (`SplineComponent.GetSplineLength` _choosedspline_2))
  (bind _returnvalue_2 (/ _returnvalue (`SplineComponent.GetNumberOfSplinePoints` _choosedspline_2)))
  (set `self.StartPointDist` (`SplineComponent.GetDistanceAlongSplineAtSplinePoint` _choosedspline (`KismetMathLibrary.FTrunc` (`SplineComponent.FindInputKeyClosestToWorldLocation` _choosedspline (`self.K2_GetActorLocation`)))))
  ; Movement along the spline
  (if (`self.Reversed`)
    (bind (_direction _alpha) (`Timeline|MoveAlong` :!via `ReverseFromEnd` :!label _label)
      (:`Update`
        (set `self.IsStopped` false)
        (if (!= _startpointdist 0.0)
          (`self.K2_SetActorLocation` (`SplineComponent.GetLocationAtDistanceAlongSpline` _choosedspline_2 (`|EaseFunction` "Linear" _alpha _returnvalue_2 _returnvalue) "World"))
          (else
            (`self.K2_SetActorLocation` (`SplineComponent.GetLocationAtDistanceAlongSpline` _choosedspline_2 (`|EaseFunction` "Linear" _alpha _startpointdist _returnvalue_2) "World")))))
      (:`Finished`
        (set `self.IsStopped` true)
        (set `self.StartPointDist` 0.0)))
    (else
      (goto _label :!via `PlayFromStart`))))

(fn `UserConstructionScript`)