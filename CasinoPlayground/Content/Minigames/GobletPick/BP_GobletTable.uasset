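; Interactable table for the goblet-pick minigame, which spawns goblets and shuffles them in pairs.
; BeginInteraction shows the game UI and mouse cursor, spawns goblets at tagged box components and binds the UI's shuffle event.
; Each shuffle picks two random goblets, seeks a spline both can use and moves them along it with a shared random direction.
; EndInteraction destroys the goblets; closest-camera and debug logic is left unconnected.
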(event `self.BeginInteraction`
  (bind _returnvalue (`GameplayStatics.GetPlayerController` 0))
  (bind _gobletspawnposref (`self.GobletSpawnPosRef`))
  (`parent.BeginInteraction`)
  (`/Engine/EditorBlueprintResources/StandardMacros.DoOnce` false :!label _label
    (:`Completed`
      ; Assign Game UI to the player
      (if (not (`Widget.IsInViewport` (stale _returnvalue_2)))
        (bind _returnvalue_2 (`|CreateWidget` "/Game/Minigames/GobletPick/UI_GobletGame.UI_GobletGame_C" _returnvalue))
        (bind _output_get (set `self.GameUI` _returnvalue_2))
        (`UserWidget.AddToViewport` _output_get 0)
        (`WidgetBlueprintLibrary.SetFocusToGameViewport`)
        (set `PlayerController.bShowMouseCursor` true _returnvalue)
        ; Get Goblet Spawn Positions
        (for (_array_element _array_index) (`self.GetComponentsByTag` "/Script/Engine.BoxComponent" "SpawnLocation")
          (`KismetArrayLibrary.Array_Add` _gobletspawnposref (`SceneComponent.K2_GetComponentToWorld` _array_element))
          ; Spawn Goblets
          (bind _returnvalue_3 (`|SpawnActorFromClass` "/Game/Minigames/GobletPick/BP_Goblet.BP_Goblet_C" (`|GetArrayItem` _gobletspawnposref _array_index) "Undefined" "MultiplyWithRoot" null null))
          (`KismetArrayLibrary.Array_Add` (`self.GobletRef`) _returnvalue_3))
        (add `/Game/Minigames/GobletPick/UI_GobletGame.Shuffle` (`self.GameUI`) (delegate `OnClickShuffle_Event`))))))

(event `self.EndInteraction`
  (bind _gobletref (`self.GobletRef`))
  ; Cleanup after EndInteraction
  (for _array_element _gobletref
    (`self.K2_DestroyActor` _array_element)
    (set `self.CorrespondingGoblet` null)
    (set `self.PickedGoblet` null))
  (`KismetArrayLibrary.Array_Clear` _gobletref)
  (goto _label :!via `Reset`))

(event `OnClickShuffle_Event`
  (bind _pickedgoblet (`self.PickedGoblet`))
  (bind _foundsplinerefs (`/Game/Minigames/GobletPick/BP_Goblet.FoundSplineRefs` (`self.CorrespondingGoblet`)))
  ; Pick Random Goblet and Path
  (set `self.PickedGoblet` (`KismetArrayLibrary.Array_Random` (`self.GobletRef`)))
  ; Find corresponding goblet and possible paths for both goblets
  (`KismetArrayLibrary.Array_RemoveItem` (`self.GobletRef`) (`self.PickedGoblet`))
  (bind _output_get (set `self.CorrespondingGoblet` (`KismetArrayLibrary.Array_Random` (`self.GobletRef`))))
  (`/Game/Minigames/GobletPick/BP_Goblet.FindPossibleSplines` _output_get)
  (`/Game/Minigames/GobletPick/BP_Goblet.FindPossibleSplines` (`self.PickedGoblet`))
  ; Find joint paths for both goblets
  (for _array_element (`/Game/Minigames/GobletPick/BP_Goblet.FoundSplineRefs` (`self.PickedGoblet`)) :!label _label_2
    (bind _output (`|GetArrayItem` _foundsplinerefs (`KismetArrayLibrary.Array_Find` _foundsplinerefs _array_element)))
    (if (== _array_element _output)
      (set `/Game/Minigames/GobletPick/BP_Goblet.ChoosedSpline` _output (`self.PickedGoblet`))
      (set `/Game/Minigames/GobletPick/BP_Goblet.ChoosedSpline` _output (`self.CorrespondingGoblet`))
      (`self.ForEachLoopBreak`)))
  ; Shuffle
  (bind _output_get_2 (set `/Game/Minigames/GobletPick/BP_Goblet.Reversed` (`KismetMathLibrary.RandomBool`) _pickedgoblet))
  (set `/Game/Minigames/GobletPick/BP_Goblet.Reversed` _output_get_2 (`self.CorrespondingGoblet`))
  (`/Game/Minigames/GobletPick/BP_Goblet.Shuffle` _pickedgoblet)
  (`/Game/Minigames/GobletPick/BP_Goblet.Shuffle` (`self.CorrespondingGoblet`))
  (`KismetArrayLibrary.Array_Add` (`self.GobletRef`) (`self.PickedGoblet`)))

(event `ForEachLoopBreak`
  ; Find joint paths for both goblets
  (goto _label_2 :!via `Break`))

(fn `UserConstructionScript`
  (`parent.UserConstructionScript`))