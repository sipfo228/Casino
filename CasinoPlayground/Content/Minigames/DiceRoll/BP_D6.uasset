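; Six-sided die for the dice roll minigame that tracks which face points up.
; Rolling moves the mesh 150 units above the first actor tagged DiceTable, setting that as relative location, and randomizes its rotation.
; Every Tick transforms each FaceNormals entry by the mesh's relative transform and dots it with up.
; The first above the threshold sets UpFace to its one-based index, otherwise zero.
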(event `self.ReceiveTick`
  (params (DeltaSeconds :type "Float (single-precision)"))
  ; Check which side is facing upwards
  (for (_array_element _array_index) (`self.FaceNormals`) :!label _label
    (set `self.UpFace` 0)
    (if (> (`KismetMathLibrary.Dot_VectorVector` (`KismetMathLibrary.TransformDirection` (`SceneComponent.GetRelativeTransform` (`self.StaticMesh`)) _array_element) (0.0 0.0 1.0)) 0.6)
      (set `self.UpFace` (+ _array_index 1))
      (`self.Break ForEachLoop`))))

(event `Break ForEachLoop`
  ; Check which side is facing upwards
  (goto _label :!via `Break`))

(event `Rolling`
  ; Rolling
  (bind _outactors (`GameplayStatics.GetAllActorsWithTag` "DiceTable"))
  (`SceneComponent.K2_SetRelativeLocation` (`self.StaticMesh`) (+ (`self.K2_GetActorLocation` (`|GetArrayItem` _outactors)) (0.0 0.0 150.0)) false false)
  (`SceneComponent.K2_SetRelativeRotation` (`self.StaticMesh`) (`KismetMathLibrary.RandomRotator` true) false false))

(fn `UserConstructionScript`)